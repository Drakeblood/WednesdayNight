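; Behavior tree service that measures the distance from the AI's controlled pawn to the actor in the TargetToFollow blackboard key.
; On search start it caches the controlled pawn, then writes the distance to the DistToTarget float key.
; Each tick repeats the write using the cached pawn and briefly prints the distance for debugging.
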(event EventReceiveSearchStartAI
  (params (OwnerController :type AI%20Controller%20Object%20Reference) (ControlledPawn :type Pawn%20Object%20Reference))
  (Variables|Default|SetControlledPawn ControlledPawn)
  (Class|BTFunctionLibrary|SetBlackboardValueasFloat (Variables|Default|GetDistToTarget) (Transformation|GetDistanceTo (Variables|Default|GetControlledPawn) (AI|BehaviorTree|GetBlackboardValueasActor (Variables|Default|GetTargetToFollow))))
  (Development|PrintString (Utilities|String|Append "Distance to target: " (Utilities|String|ToString(Float) (Transformation|GetDistanceTo (Variables|Default|GetControlledPawn) (AI|BehaviorTree|GetBlackboardValueasActor (Variables|Default|GetTargetToFollow))))) true true "(R=0.000000,G=0.660000,B=1.000000,A=1.000000)" 0.1))

(event EventReceiveTickAI
  (params (OwnerController :type AI%20Controller%20Object%20Reference) (ControlledPawn :type Pawn%20Object%20Reference) (DeltaSeconds :type Float%20%28single-precision%29))
  (bind _targettofollow (Variables|Default|GetTargetToFollow))
  (bind _returnvalue (AI|BehaviorTree|GetBlackboardValueasActor _targettofollow))
  (bind _returnvalue_2 (Transformation|GetDistanceTo (Variables|Default|GetControlledPawn) _returnvalue))
  (Class|BTFunctionLibrary|SetBlackboardValueasFloat (Variables|Default|GetDistToTarget) _returnvalue_2)
  (Development|PrintString (Utilities|String|Append "Distance to target: " (Utilities|String|ToString(Float) _returnvalue_2)) true true "(R=0.000000,G=0.660000,B=1.000000,A=1.000000)" 0.1))