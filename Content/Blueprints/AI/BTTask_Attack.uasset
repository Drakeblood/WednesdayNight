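; Behavior tree task that makes an AI-controlled BP_CharacterBase perform an attack ability.
; It looks up the ability by AttackTag on the character's Abilities, binds to its end event, then activates it.
; The task finishes successfully when the ability ends and fails if the pawn is not a BP_CharacterBase.
; A check for already active abilities is present but disconnected, so it never runs.
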(event Custom|OnAbilityEnded_Event
  (AI|BehaviorTree|FinishExecute true))

(event EventReceiveExecuteAI
  (params (OwnerController :type AI%20Controller%20Object%20Reference) (ControlledPawn :type Pawn%20Object%20Reference))
  (bind _asbp_character_base (Utilities|Casting|CastToBP_CharacterBase ControlledPawn)
    (:then
      (EventDispatchers|AssignOnAbilityEnded (Default|GetAbilitybyTag (Variables|/Game/Blueprints/Character/BP_CharacterBase.BP_CharacterBase_C|GetAbilities _asbp_character_base) (Variables|Default|GetAttackTag)) (delegate Custom|OnAbilityEnded_Event))
      (Default|ActivateAbility (Variables|/Game/Blueprints/Character/BP_CharacterBase.BP_CharacterBase_C|GetAbilities _asbp_character_base) (Default|GetAbilitybyTag (Variables|/Game/Blueprints/Character/BP_CharacterBase.BP_CharacterBase_C|GetAbilities _asbp_character_base) (Variables|Default|GetAttackTag))))
    (:CastFailed
      (AI|BehaviorTree|FinishExecute false))))