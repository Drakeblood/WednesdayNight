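; Behavior tree decorator that passes when the blackboard Target actor lies within a cone in front of the AI-controlled pawn.
; It takes the arccosine of the dot product between the pawn's forward vector and the normalized direction to the target, then compares the result in degrees to Angle, which acts as the cone's half-angle.
; A debug print of the computed angle is left disconnected.
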(fn PerformConditionCheckAI
  (params (OwnerController :type AI%20Controller%20Object%20Reference) (ControlledPawn :type Pawn%20Object%20Reference))
  (bind _target (Variables|Default|GetTarget))
  (bind _returnvalue (AI|BehaviorTree|GetBlackboardValueasActor _target))
  (Utilities|IsValid _returnvalue
    (:Is%20Valid
      (return (<= (Class|KismetMathLibrary|DegAcos (Math|Vector|DotProduct (Class|KismetMathLibrary|VectorNormalUnsafe (- (Transformation|GetActorLocation _returnvalue) (Transformation|GetActorLocation ControlledPawn))) (Transformation|GetActorForwardVector ControlledPawn))) (Variables|Default|GetAngle))))))