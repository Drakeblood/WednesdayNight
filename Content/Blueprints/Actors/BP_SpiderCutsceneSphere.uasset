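; BP_SpiderCutsceneSphere is a trigger sphere that starts the spider cutscene once, when the hero enters it.
; On BeginPlay it reads the played flag from the game instance's save game.
; On the first hero overlap it disables the hero's input, sets the flag locally and on the save object, and calls PlaySpider on the player controller's HUD widget.
; It neither re-enables input nor writes the save to disk itself.
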(event OnComponentBeginOverlap(Sphere)
  (params (OverlappedComponent :type Primitive%20Component%20Object%20Reference) (OtherActor :type Actor%20Object%20Reference) (OtherComp :type Primitive%20Component%20Object%20Reference) (OtherBodyIndex :type Integer) (bFromSweep :type Boolean) (SweepResult :type Hit%20Result%20Structure%20%28by%20ref%29))
  (bind _asbp_hero_character (Utilities|Casting|CastToBP_HeroCharacter OtherActor))
  (if (not (Variables|Default|GetPlayed))
    (Input|DisableInput _asbp_hero_character 0)
    (Variables|Default|SetPlayed true)
    (bind _asbp_game_instance (Utilities|Casting|CastToBP_GameInstance (Game|GetGameInstance))
      (:then
        (bind _savegame (Variables|/Game/Blueprints/System/BP_GameInstance.BP_GameInstance_C|GetSaveGame _asbp_game_instance)
          (:then
            (Variables|/Game/Blueprints/BP_SaveGame.BP_SaveGame_C|SetSpiderCutscenePlayed _savegame true))
          (:else
            _)))
      (:CastFailed
        _))
    (bind _asbp_player_controller (Utilities|Casting|CastToBP_PlayerController (Pawn|GetController _asbp_hero_character)))
    (bind _playerhudwidget (Variables|/Game/Blueprints/Player/BP_PlayerController.BP_PlayerController_C|GetPlayerHUDWidget _asbp_player_controller)
      (:then
        (Default|PlaySpider _playerhudwidget))
      (:else))))

(event EventBeginPlay
  (bind _asbp_game_instance (Utilities|Casting|CastToBP_GameInstance (Game|GetGameInstance)))
  (bind _savegame (Variables|/Game/Blueprints/System/BP_GameInstance.BP_GameInstance_C|GetSaveGame _asbp_game_instance)
    (:then
      (Variables|Default|SetPlayed (Variables|/Game/Blueprints/BP_SaveGame.BP_SaveGame_C|GetSpiderCutscenePlayed _savegame)))
    (:else)))

(fn ConstructionScript)