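; BP_ActivatableGate is a gate actor that moves to an open or offset position when activated, then returns on its own.
; BeginPlay caches the start location and converts the local OnActivateLocation offset into a world-space target.
; Activate plays a timeline that lerps the actor between both points without sweeping, then reverses it after a short delay.
; An Active flag blocks retriggering during the forward move and stops the reverse pass from looping.
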(event EventBeginPlay
  (Variables|Default|SetOriginalLocation (Transformation|GetActorLocation))
  (Variables|Default|SetOnActivateWorldLocation (Math|Transform|TransformLocation (Transformation|GetActorTransform) (Variables|Default|GetOnActivateLocation))))

(event EventActivate
  (params (Instigator :type Pawn%20Object%20Reference))
  (if (not (Variables|Default|GetActive))
    (Variables|Default|SetActive true)
    (bind _alpha (Timeline|Timeline_0 Play)
      (:Update
        (Transformation|SetActorLocation (Math|Vector|Lerp(Vector) (Variables|Default|GetOriginalLocation) (Variables|Default|GetOnActivateWorldLocation) _alpha) false false))
      (:Finished
        (if (Variables|Default|GetActive)
          (Variables|Default|SetActive false)
          (Utilities|FlowControl|Delay 3.0)
          (Timeline|Timeline_0 ReverseFromEnd))))))

(fn ConstructionScript)