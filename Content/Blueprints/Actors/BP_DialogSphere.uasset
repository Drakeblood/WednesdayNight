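; BP_DialogSphere is a trigger actor that plays a sequence of dialog sounds when the hero character enters its sphere.
; The overlap starts the first entry of the Dialogs array on its audio component and binds the finished event.
; Each finish plays the next clip by index, then unbinds once the array is exhausted.
; The index is never reset, and the overlap has no guard against retriggering.
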(event OnComponentBeginOverlap(Sphere)
  (params (OverlappedComponent :type Primitive%20Component%20Object%20Reference) (OtherActor :type Actor%20Object%20Reference) (OtherComp :type Primitive%20Component%20Object%20Reference) (OtherBodyIndex :type Integer) (bFromSweep :type Boolean) (SweepResult :type Hit%20Result%20Structure%20%28by%20ref%29))
  (bind _audio (Variables|Default|GetAudio))
  (Utilities|Casting|CastToBP_HeroCharacter OtherActor)
  (EventDispatchers|AssignOnAudioFinished _audio (delegate Custom|OnAudioFinished_Event))
  (Audio|Components|Audio|SetSound _audio (Utilities|Array|Get(acopy) (Variables|Default|GetDialogs)))
  (Math|Integer|IncrementInt (Variables|Default|GetCurrentIndex)
    (:%20%20
      (Audio|Components|Audio|Play _audio 0.0))))

(event Custom|OnAudioFinished_Event
  (bind _audio (Variables|Default|GetAudio))
  (if (< (Variables|Default|GetCurrentIndex) (Utilities|Array|Length (Variables|Default|GetDialogs)))
    (Audio|Components|Audio|SetSound _audio (Utilities|Array|Get(acopy) (Variables|Default|GetDialogs) (Variables|Default|GetCurrentIndex)))
    (Audio|Components|Audio|Play _audio 0.0)
    (Math|Integer|IncrementInt (Variables|Default|GetCurrentIndex))
    (else
      (EventDispatchers|UnbindEventfromOnAudioFinished (Variables|Default|GetAudio) (delegate Custom|OnAudioFinished_Event)))))

(fn ConstructionScript)