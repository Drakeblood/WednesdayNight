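; BP_MultiShootable is a linked target that triggers other actors when its whole group is hit almost simultaneously.
; Any overlap with its Sphere sets Active for a brief window, using a latent Delay to clear it.
; Without waiting for that delay, CheckActivation tests whether every actor in OtherShootables is also Active.
; If so, it sends ActivateMessage to each entry in Activatables, passing the overlapping actor's instigator.
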(event OnComponentBeginOverlap(Sphere)
  (params (OverlappedComponent :type Primitive%20Component%20Object%20Reference) (OtherActor :type Actor%20Object%20Reference) (OtherComp :type Primitive%20Component%20Object%20Reference) (OtherBodyIndex :type Integer) (bFromSweep :type Boolean) (SweepResult :type Hit%20Result%20Structure%20%28by%20ref%29))
  (Utilities|FlowControl|Sequence
    (:then_0
      (Variables|Default|SetActive true)
      (Utilities|FlowControl|Delay 0.3)
      (Variables|Default|SetActive false))
    (:then_1
      (if (CallFunction|CheckActivation)
        (for _array_element (Variables|Default|GetActivatables)
          (Class|BPIActivatable|Activate(Message) _array_element (Game|GetInstigator OtherActor)))))))

(event EventBeginPlay)

(event Collision|EventActorBeginOverlap
  (params (OtherActor :type Actor%20Object%20Reference)))

(event EventTick
  (params (DeltaSeconds :type Float%20%28single-precision%29)))

(fn ConstructionScript)

(fn CheckActivation
  (for _array_element (Variables|Default|GetOtherShootables)
    (if (not (Variables|BP_MultiShootable_C|GetActive _array_element))
      (return false)))
  (return true))