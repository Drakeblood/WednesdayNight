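; Ice golem boss enemy with a firewall hazard, spider minion spawning and a stun window opened by ultimate hits, reusing spider montages.
; Firewall activation nudges the component to refresh overlaps, damaging each actor once per activation.
; An ultimate hit while susceptible makes it damageable until the stun montage ends.
; BeginPlay only runs a delayed death-montage test; parent initialization and weapon attachment are disconnected.
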(event OnComponentBeginOverlap(Firewall)
  (params (OverlappedComponent :type Primitive%20Component%20Object%20Reference) (OtherActor :type Actor%20Object%20Reference) (OtherComp :type Primitive%20Component%20Object%20Reference) (OtherBodyIndex :type Integer) (bFromSweep :type Boolean) (SweepResult :type Hit%20Result%20Structure%20%28by%20ref%29))
  (if (!= OtherActor self)
    (bind _returnvalue (Utilities|Array|AddUnique (Variables|Default|GetHitActors) OtherActor))
    (if (!= _returnvalue -1)
      (Game|Damage|ApplyDamage OtherActor (Variables|Default|GetFirewallDamage) 0 self))))

(event Custom|ActivateFirewall
  (bind _firewall (Variables|Default|GetFirewall))
  (bind _relativelocation (Variables|/Script/Engine.SceneComponent|GetRelativeLocation _firewall))
  (Variables|/Script/Engine.PrimitiveComponent|SetbGenerateOverlapEvents (Variables|Default|GetFirewall) true)
  (bind _output_get (Variables|Default|SetOriginalRelative%20Location _relativelocation))
  (Transformation|SetRelativeLocation _firewall (+ _relativelocation 1.0) false false)
  (Transformation|SetRelativeLocation _firewall _output_get false false)
  (Utilities|Array|Clear (Variables|Default|GetHitActors)))

(event Custom|DeactivateFirewall
  (Variables|/Script/Engine.PrimitiveComponent|SetbGenerateOverlapEvents (Variables|Default|GetFirewall) false))

(event Custom|SpawnMinions
  (for _array_element (Variables|Default|GetMinionSpawnPoints)
    (bind _returnvalue (Game|SpawnActorfromClass "/Game/Blueprints/Enemy/BP_Spider.BP_Spider_C" (Math|Transform|MakeTransform (Math|Transform|TransformLocation (Transformation|GetActorTransform) _array_element) (Transformation|GetActorRotation) "1,1,1") "AlwaysSpawn" (Components|GetOwner) 0))
    (Pawn|SpawnDefaultController _returnvalue)))

(event Custom|MakeSusceptible
  (params (Susceptible :type Boolean))
  (Variables|Default|SetUltimateDamageable Susceptible))

(event EventOnUltimateHit
  (|CallParentFunction)
  (if (Variables|Default|GetUltimateDamageable)
    (Variables|Default|SetUltimateDamageable false)
    (Variables|Default|SetDamageable true)
    (Animation|Montage|PlayMontage (Variables|Character|GetMesh) "/Game/Animations/Boss/AM_Spider_Stun.AM_Spider_Stun"
      (:OnCompleted
        _)
      (:OnBlendOut
        _)
      (:OnInterrupted
        _))
    (Variables|Default|SetDamageable false)
    (Variables|Default|SetUltimateDamageable true)))

(event EventBeginPlay
  (Utilities|FlowControl|Delay 3.0)
  (Animation|Montage|PlayMontage (Variables|Character|GetMesh) "/Game/InfinityBladeAdversaries/Enemy/Enemy_Frost_Giant/Enemy_Frost_Giant_All_Animation/AM_IceGolemDeath.AM_IceGolemDeath"
    (:then
      (Development|PrintString "Hello"))))

(fn ConstructionScript
  (|CallParentFunction))

(fn CreateAttackAbility
  (params (Tag :type Gameplay%20Tag%20Structure))
  (bind _returnvalue (Game|ConstructObjectfromClass "/Game/Blueprints/Abilities/BP_AttackAbility.BP_AttackAbility_C" self))
  (|SwitchGameplayTag Tag
    (:Enemy.Spider.Attack.Claws
      (LocalVariables|SetMontageToSet "/Game/Animations/Boss/AM_Spider_Melee.AM_Spider_Melee"))
    (:Enemy.Spider.Attack.Charge
      (LocalVariables|SetMontageToSet "/Game/Animations/Boss/AM_Spider_Charge.AM_Spider_Charge")))
  (Variables|/Game/Blueprints/Abilities/BP_AttackAbility.BP_AttackAbility_C|SetMontageToPlay _returnvalue (LocalVariables|GetMontageToSet))
  (return _returnvalue))