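; BP_Worm is an enemy Blueprint that spawns a worm weapon on its jaw socket and can perform a lunging jump attack.
; JumpAttack turns toward the player, then a timeline drives a swept lerp along its velocity (or facing, if stationary) while the weapon is active.
; On landing it deactivates the weapon and restores walk-speed velocity.
; CreateAttackAbility builds attack abilities, mapping Spider claw and charge tags to Spider montages.
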(event Custom|JumpAttack
  (bind _returnvalue (Transformation|GetVelocity))
  (bind _charactermovement (Variables|Character|GetCharacterMovement))
  (Transformation|SetActorRotation (Math|Rotator|FindLookatRotation (Transformation|GetActorLocation) (Transformation|GetActorLocation (Game|Player|GetPlayerPawn 0))))
  (bind _output_get (Variables|Default|SetJumpStartLocation (Transformation|GetActorLocation)))
  (Variables|Default|SetJumpTargetLocation (+ _output_get (* (select (Math|Vector|VectorIsNearlyZero _returnvalue) (Transformation|GetActorForwardVector) (Math|Vector|Normalize _returnvalue)) (Variables|Default|GetJumpLength))))
  (Physics|AddImpulse (Variables|Character|GetCharacterMovement) "0, 0,100.000000" false)
  (CallFunction|ActivateWeapon)
  (bind _newtrack_0 (Timeline|JumpTimeline PlayFromStart)
    (:Update
      (Transformation|SetActorLocation (Math|Vector|Lerp(Vector) (Variables|Default|GetJumpStartLocation) (Variables|Default|GetJumpTargetLocation) _newtrack_0) true false))
    (:Finished
      (Variables|/Script/Engine.MovementComponent|SetVelocity _charactermovement (* (Math|Vector|Normalize (Transformation|GetVelocity)) (Variables|/Script/Engine.CharacterMovementComponent|GetMaxWalkSpeed _charactermovement)))
      (CallFunction|DeactivateWeapon))))

(event EventBeginPlay
  (bind _self self)
  (|CallParentFunction)
  (bind _returnvalue (Game|SpawnActorfromClass "/Game/Blueprints/Weapon/Spider/BP_WeaponWorm.BP_WeaponWorm_C" (Math|Transform|MakeTransform "0, 0, 0" "0, 0, 0" "1,1,1") "Undefined" _self _self))
  (Utilities|Array|Add (Variables|Default|GetCurrentWeapons) _returnvalue)
  (Transformation|AttachComponentToComponent _returnvalue (Variables|Character|GetMesh) "JawSocket" "SnapToTarget" "SnapToTarget" "KeepRelative" true))

(fn ConstructionScript
  (|CallParentFunction))

(fn CreateAttackAbility
  (params (Tag :type Gameplay%20Tag%20Structure))
  (bind _returnvalue (Game|ConstructObjectfromClass "/Game/Blueprints/Abilities/BP_AttackAbility.BP_AttackAbility_C" self))
  (|SwitchGameplayTag Tag
    (:Enemy.Spider.Attack.Claws
      (LocalVariables|SetMontageToSet "/Game/Animations/Boss/AM_Spider_Melee.AM_Spider_Melee"))
    (:Enemy.Spider.Attack.Charge
      (LocalVariables|SetMontageToSet "/Game/Animations/Boss/AM_Spider_Charge.AM_Spider_Charge")))
  (Variables|/Game/Blueprints/Abilities/BP_AttackAbility.BP_AttackAbility_C|SetMontageToPlay _returnvalue (LocalVariables|GetMontageToSet))
  (return _returnvalue))