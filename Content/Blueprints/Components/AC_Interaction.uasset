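; AC_Interaction is an actor component that makes its owner interactable, with a prompt shown while it is registered.
; RegisterInteractable lazily adds a screen-space widget component holding WBP_Interaction and shows it when CanInteract allows; UnregisterInteractable hides it.
; Interact requires CanInteract, plus owner approval if it implements BPI_Interactable, then calls OnInteract and has a BP_HeroCharacter interacter unregister the interactable.
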(fn RegisterInteractable
  (Variables|Default|GetWidgetComponent
    (:then
      _)
    (:else
      (bind _returnvalue (Game|AddComponentbyClass (Components|GetOwner) "/Script/UMG.WidgetComponent" false))
      (bind _output_get (Variables|Default|SetWidgetComponent _returnvalue))
      (Class|WidgetComponent|SetWidgetSpace _output_get "Screen")
      (bind _returnvalue_2 (UserInterface|CreateWidget "/Game/Blueprints/UI/WBP_Interaction.WBP_Interaction_C"))
      (UserInterface|SetWidget _output_get _returnvalue_2)))
  (if (not (Class|WidgetComponent|IsWidgetVisible (Variables|Default|GetWidgetComponent)))
    (Rendering|SetVisibility (Variables|Default|GetWidgetComponent) (Variables|Default|GetCanInteract) false)))

(fn UnregisterInteractable
  (Variables|Default|GetWidgetComponent
    (:then
      (Rendering|SetVisibility (Variables|Default|GetWidgetComponent) false false))
    (:else)))

(fn Interact
  (params (Interacter :type Actor%20Object%20Reference))
  (bind _returnvalue (Components|GetOwner))
  (bind _caninteract (Variables|Default|GetCanInteract))
  (if (Utilities|DoesObjectImplementInterface _returnvalue "/Game/Blueprints/Interfaces/BPI_Interactable.BPI_Interactable_C")
    (bind _available (Class|BPIInteractable|IsAvailableforInteraction(Message) _returnvalue Interacter))
    (if (and _available _caninteract)
      (Default|CallOnInteract Interacter :!label _label)
      (bind _asbp_hero_character (Utilities|Casting|CastToBP_HeroCharacter Interacter))
      (Default|UnregisterInteractable _asbp_hero_character))
    (elif _caninteract
      (goto _label))))