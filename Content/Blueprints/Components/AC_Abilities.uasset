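; Actor component that manages abilities for its owning actor.
; On BeginPlay it constructs each class in InitialAbilities with the owner as outer, maps it by AbilityTag for lookup and calls AbilityAdded.
; ActivateAbility starts a valid, inactive ability, sets IsAnyAbilityActive, then binds to its ended event and returns success.
; The IsAnyAbilityActive guard is disconnected, so the flag does not block overlapping abilities.
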(event Custom|OnAbilityEndedEvent
  (Variables|Default|SetIsAnyAbilityActive false))

(event EventBeginPlay
  (for _array_element (Variables|Initial|GetInitialAbilities)
    (bind _returnvalue (Game|ConstructObjectfromClass _array_element (Components|GetOwner)))
    (Utilities|Map|Add (Variables|Abilities|GetAbilities) (Variables|/Game/Blueprints/Abilities/BP_AbilityBase.BP_AbilityBase_C|GetAbilityTag _returnvalue) _returnvalue)
    (Default|AbilityAdded _returnvalue)))

(fn GetAbilitybyTag
  (params (Tag :type Gameplay%20Tag%20Structure%20%28by%20ref%29))
  (return (.Value (Utilities|Map|Find (Variables|Abilities|GetAbilities) Tag))))

(fn ActivateAbility
  (params (Ability :type BP%20Ability%20Base%20Object%20Reference%20%28by%20ref%29))
  (Utilities|IsValid Ability
    (:Is%20Valid
      (if (not (Variables|/Game/Blueprints/Abilities/BP_AbilityBase.BP_AbilityBase_C|GetIsActive Ability))
        (Default|ActivateAbility Ability)
        (Variables|Default|SetIsAnyAbilityActive true)
        (EventDispatchers|BindEventtoOnAbilityEnded Ability (EventDispatchers|CreateEvent :!event Custom|OnAbilityEndedEvent))
        (return true)
        (else
          _)))
    (:Is%20Not%20Valid
      _))
  (return false))