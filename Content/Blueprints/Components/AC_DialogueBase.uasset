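; Base dialogue component that runs branching, voiced conversations through the player HUD's dialogue widget.
; The empty Dialogue function serves as the script, calling AddDialogue for each line.
; Each progression replays Dialogue from the start; AddDialogue returns saved choices for answered indices, otherwise displays the line and plays its sound on the owner's AudioComponent.
; Choices, or audio completion on auto-pass lines, record progress and trigger another replay.
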(event Custom|AutoPassThrough
  (CallFunction|UpdateSelectedOption (Variables|Default|GetDialogueIndex) (Class|KismetSystemLibrary|MakeLiteralInteger)))

(event EventBeginPlay
  (Variables|Default|SetAudioComponent (Actor|GetComponentbyClass (Components|GetOwner) "/Script/Engine.AudioComponent")))

(fn OpenConversation
  (bind _asbp_player_controller (Utilities|Casting|CastToBP_PlayerController (Game|GetPlayerController 0)))
  (bind _playerhudwidget (Variables|/Game/Blueprints/Player/BP_PlayerController.BP_PlayerController_C|GetPlayerHUDWidget _asbp_player_controller)
    (:then
      (bind _output_get (Variables|Default|SetDialogueWidget (Variables|/Game/Blueprints/UI/WBP_HUD.WBP_HUD_C|GetWBP_Dialogue _playerhudwidget)))
      (Variables|/Game/Blueprints/UI/WBP_Dialogue.WBP_Dialogue_C|SetOwningDialogueComponent _output_get self)
      (Widget|SetRenderOpacity _output_get 1.0)
      (CallFunction|ProgressDialogue))
    (:else)))

(fn CloseConversation
  (bind _returnvalue (Game|GetPlayerController 0))
  (Widget|SetRenderOpacity (Variables|Default|GetDialogueWidget) 0.0)
  (Input|SetInputModeGameOnly _returnvalue)
  (Variables|/Script/Engine.PlayerController|SetbShowMouseCursor _returnvalue false)
  (Audio|Components|Audio|Stop (Variables|Default|GetAudioComponent))
  (EventDispatchers|UnbindEventfromOnAudioFinished (Variables|Default|GetAudioComponent) (EventDispatchers|CreateEvent :!event Custom|AutoPassThrough)))

(fn ProgressDialogue
  (Variables|Default|SetDialogueIndex -1)
  (CallFunction|Dialogue))

(fn Dialogue)

(fn AddDialogue
  (params (Speaker :type Text) (Dialogue :type Text) (OptionsText :type Array%20of%20Texts) (Sound :type Sound%20Wave%20Object%20Reference) (AutoPassThrough :type Boolean))
  (bind _dialogueprogress (Variables|Default|GetDialogueProgress))
  (bind _dialogueindex (Variables|Default|GetDialogueIndex))
  (bind (_value _returnvalue) (Utilities|Map|Find _dialogueprogress _dialogueindex))
  (Math|Integer|IncrementInt (Variables|Default|GetDialogueIndex)
    (:%20%20
      (if _returnvalue
        (return "NewEnumerator0" _value)
        (else
          (Default|UpdateDialogueText (Variables|Default|GetDialogueWidget) (Variables|Default|GetDialogueIndex) Speaker Dialogue OptionsText)
          (Audio|Components|Audio|Stop (Variables|Default|GetAudioComponent))
          (Audio|Components|Audio|SetSound (Variables|Default|GetAudioComponent) Sound)
          (Audio|Components|Audio|Play (Variables|Default|GetAudioComponent) 0.0)
          (if AutoPassThrough
            (EventDispatchers|BindEventtoOnAudioFinished (Variables|Default|GetAudioComponent) (EventDispatchers|CreateEvent :!event Custom|AutoPassThrough))
            (else
              (EventDispatchers|UnbindEventfromOnAudioFinished (Variables|Default|GetAudioComponent) (EventDispatchers|CreateEvent :!event Custom|AutoPassThrough))))
          (return "NewEnumerator1" 0))))))

(fn UpdateSelectedOption
  (params (ProgressIndex :type Integer%20%28by%20ref%29) (OptionIndex :type Integer%20%28by%20ref%29))
  (Utilities|Map|Add (Variables|Default|GetDialogueProgress) ProgressIndex OptionIndex)
  (CallFunction|ProgressDialogue))

(fn ClearDialogueProgress
  (Utilities|Map|Clear (Variables|Default|GetDialogueProgress)))

(fn RemoveDialogueProgress
  (params (ProgressSteps :type Integer))
  (for _index (range 0 ProgressSteps)
    (Utilities|Map|Remove (Variables|Default|GetDialogueProgress) (- (Variables|Default|GetDialogueIndex) _index))))

(fn SetDialogueTreeIndex
  (params (DialogueTreeIndex :type Integer))
  (Variables|Default|SetDialogueTreeIndex DialogueTreeIndex)
  (CallFunction|ClearDialogueProgress))