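; AC_Attributes is an attributes component that holds Health and MaxHealth and exposes getters and setters for both.
; Each setter acts only when the new value differs, then fires OnHealthChanged or OnMaxHealthChanged with the value and the component itself.
; SetMaxHealth writes the new value into Health and broadcasts that, leaving MaxHealth itself unchanged.
; SetHealth applies no clamping against MaxHealth.
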(fn SetHealth
  (params (NewHealth :type Float%20%28single-precision%29))
  (if (!= NewHealth (Variables|Attributes|GetHealth))
    (bind _output_get (Variables|Attributes|SetHealth NewHealth))
    (Default|CallOnHealthChanged _output_get self)))

(fn SetMaxHealth
  (params (NewMaxHealth :type Float%20%28single-precision%29))
  (if (!= NewMaxHealth (Variables|Attributes|GetMaxHealth))
    (bind _output_get (Variables|Attributes|SetHealth NewMaxHealth))
    (Default|CallOnMaxHealthChanged _output_get self)))

(fn GetHealth
  (return (Variables|Attributes|GetHealth)))

(fn GetMaxHealth
  (return (Variables|Attributes|GetMaxHealth)))