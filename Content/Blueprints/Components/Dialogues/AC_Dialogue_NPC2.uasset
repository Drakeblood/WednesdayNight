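; Dialogue component holding a linear, voiced Polish conversation in which an NPC tells the player about its homeland Ossarion and the world of Nidavelirr.
; The Dialogue override chains AddDialogue calls through their Pass Through state, alternating single-option player prompts, auto-advancing player lines and NPC replies.
; The last step clears dialogue progress and closes the conversation.
; The speaker is labelled NPC1 despite the asset's NPC2 name.
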(event EventBeginPlay
  (|CallParentFunction) ; This node is disabled and will not be called.\nDrag off pins to build functionality.
)

(event EventTick
  (params (DeltaSeconds :type Float%20%28single-precision%29))
  (|CallParentFunction DeltaSeconds) ; This node is disabled and will not be called.\nDrag off pins to build functionality.
)

(fn Dialogue
  (bind _array (Utilities|Array|MakeArray "Hej, Jesteś... stąd?"))
  (bind _array_2 (Utilities|Array|MakeArray "Czy wiesz coś o tym świecie?"))
  (bind _array_3 (Utilities|Array|MakeArray "Dziękuje"))
  (|CallParentFunction)
  (bind (_dialoguestate _optionindex) (CallFunction|AddDialogue "" "" _array 0 false))
  (switch Utilities|FlowControl|Switch|SwitchonE_DialogueState _dialoguestate
    (:NewEnumerator0
      (bind _dialoguestate_2 (CallFunction|AddDialogue "" (Utilities|Array|Get(acopy) _array _optionindex) (Utilities|Array|MakeArray "[dalej]") "/Game/Assets/Dubbing/Hej__Jesteś…___stąd.Hej__Jesteś…___stąd" true))
      (switch Utilities|FlowControl|Switch|SwitchonE_DialogueState _dialoguestate_2
        (:NewEnumerator0
          (bind _dialoguestate_3 (CallFunction|AddDialogue "NPC1" "Nie, jestem z Ossarionu. To miejsce, gdzie większość mieszkańców jest... no właśnie, jak mnie widzisz. Nasz świat jest pełen ciemności i niebezpieczeństw. Mamy niekończące się labirynty, pełne zagadek i pułapek. Wszędzie panuje ciemność, a jedynym źródłem światła są ognie i latarnie." _array_2 "/Game/Assets/Dubbing/Skeletron.Skeletron" false))
          (switch Utilities|FlowControl|Switch|SwitchonE_DialogueState _dialoguestate_3
            (:NewEnumerator0
              (bind _dialoguestate_4 (CallFunction|AddDialogue "" (Utilities|Array|Get(acopy) _array_2) (Utilities|Array|MakeArray "[dalej]") "/Game/Assets/Dubbing/Czy_wiesz_coś_o_tym_świecie.Czy_wiesz_coś_o_tym_świecie" true))
              (switch Utilities|FlowControl|Switch|SwitchonE_DialogueState _dialoguestate_4
                (:NewEnumerator0
                  (bind _dialoguestate_5 (CallFunction|AddDialogue "NPC1" "Nidavelirr to świat, który łączy wiele różnych wymiarów, światów i epok w jednym miejscu. Jest to miejsce, gdzie spotyka się wiele różnych istot, które przybywają z różnych światów, ale tajemnicą zostaje w jaki sposób wszyscy tu trafiają. Nidavelirr to ogromny świat, który rozciąga się na niezwykle rozległych przestrzeniach, pełnych gór, dolin, lasów i pustyń. Jednym z najbardziej tajemniczych miejsc na Nidavelirr jest zaginiona cywilizacja, o której mówi się, że była jedną z najpotężniejszych w historii świata. Niewielu wie, co się z nią stało i gdzie się podziała. Przez kilka lat ja z grupą poszukiwaczy przeszukujemy każdy kąt Nidavelirru, aby odkryć tę tajemnicę i poznać historię tego niezwykłego świata, ale wszystko na marne." _array_3 "/Game/Assets/Dubbing/Skeletron1_2.Skeletron1_2" false))
                  (switch Utilities|FlowControl|Switch|SwitchonE_DialogueState _dialoguestate_5
                    (:NewEnumerator0
                      (bind _dialoguestate_6 (CallFunction|AddDialogue "" (Utilities|Array|Get(acopy) _array_3) (Utilities|Array|MakeArray "[dalej]") "/Game/Assets/Dubbing/Dziękuję__1_.Dziękuję__1_" true))
                      (switch Utilities|FlowControl|Switch|SwitchonE_DialogueState _dialoguestate_6
                        (:NewEnumerator0
                          (CallFunction|ClearDialogueProgress)
                          (CallFunction|CloseConversation))))))))))))))