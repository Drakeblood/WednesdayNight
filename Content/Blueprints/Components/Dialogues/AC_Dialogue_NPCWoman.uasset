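; Dialogue component for the elderly woman NPC ("Starsza Pani"), holding her Polish conversation with the player about the villagers' backstory.
; The Dialogue override chains parent AddDialogue calls, advancing on each Pass Through state, with voice clips and auto-advancing player replies.
; Midway, a MoviePlayed flag lets the player controller's HUD widget play the prologue only once.
; The final line calls RemoveDialogueProgress and closes the conversation.
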(event EventBeginPlay
  (|CallParentFunction))

(event EventTick
  (params (DeltaSeconds :type Float%20%28single-precision%29))
  (|CallParentFunction DeltaSeconds) ; This node is disabled and will not be called.\nDrag off pins to build functionality.
)

(fn Dialogue
  (bind _array (Utilities|Array|MakeArray "Naprawdę? Dziękuję"))
  (|CallParentFunction)
  (bind (_dialoguestate _optionindex) (CallFunction|AddDialogue "Starsza Pani" "Witam cię podróżniczko, tu znajdziesz odpowiedź na pytanie, które cię tak bardzo interesuje." _array "/Game/Assets/Dubbing/Pani1.Pani1" false))
  (switch Utilities|FlowControl|Switch|SwitchonE_DialogueState _dialoguestate
    (:NewEnumerator0
      (bind _dialoguestate_2 (CallFunction|AddDialogue "" (Utilities|Array|Get(acopy) _array _optionindex) (Utilities|Array|MakeArray "[dalej]") "/Game/Assets/Dubbing/ja1.ja1" true))
      (switch Utilities|FlowControl|Switch|SwitchonE_DialogueState _dialoguestate_2
        (:NewEnumerator0
          (Utilities|FlowControl|Sequence
            (:then_0
              (if (not (Variables|Default|GetMoviePlayed))
                (Variables|Default|SetMoviePlayed true)
                (bind _asbp_player_controller (Utilities|Casting|CastToBP_PlayerController (Game|GetPlayerController 0)))
                (bind _playerhudwidget (Variables|/Game/Blueprints/Player/BP_PlayerController.BP_PlayerController_C|GetPlayerHUDWidget _asbp_player_controller)
                  (:then
                    (Default|PlayProlog _playerhudwidget))
                  (:else))))
            (:then_1
              (bind _dialoguestate_3 (CallFunction|AddDialogue "" "" (Utilities|Array|MakeArray "Dziękuję, że pani podzieliła się tą historią...") 0 false))
              (switch Utilities|FlowControl|Switch|SwitchonE_DialogueState _dialoguestate_3
                (:NewEnumerator0
                  (bind _dialoguestate_4 (CallFunction|AddDialogue "" "Dziękuję, że pani podzieliła się tą historią.Teraz rozumiem dlaczego wszyscy mieszkańcy tak podejrzanie na mnie się gapili. Chciałabym pomóc wam w tej sytuacji.  Proszę, powiedzcie w którą stronę mam iść by tam trafić?" (Utilities|Array|MakeArray "[dalej]") "/Game/Assets/Dubbing/ja1_2.ja1_2" true))
                  (switch Utilities|FlowControl|Switch|SwitchonE_DialogueState _dialoguestate_4
                    (:NewEnumerator0
                      (bind _dialoguestate_5 (CallFunction|AddDialogue "Starsza Pani" "..." (Utilities|Array|MakeArray "[koniec]") 0 false))
                      (switch Utilities|FlowControl|Switch|SwitchonE_DialogueState _dialoguestate_5
                        (:NewEnumerator0
                          (CallFunction|RemoveDialogueProgress)
                          (CallFunction|CloseConversation))))))))))))))