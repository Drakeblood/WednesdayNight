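; Dialogue component for the second conversation with the Mysterious NPC, who offers the player help in exchange for a defeated spider's skin, voiced in Polish.
; Chained AddDialogue nodes branch on the yes/no answer.
; Accepting records the speaker in the SaveGame and, unless already rewarded, applies the hero's Rogue skin and adds a key; refusing clears dialogue progress.
; BeginPlay reads that saved flag to restore the reward state and dialogue progress.
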(event EventBeginPlay
  (|CallParentFunction)
  (bind _asbp_game_instance (Utilities|Casting|CastToBP_GameInstance (Game|GetGameInstance)))
  (bind _savegame (Variables|/Game/Blueprints/System/BP_GameInstance.BP_GameInstance_C|GetSaveGame _asbp_game_instance)
    (:then
      (if (.Value (Utilities|Map|Find (Variables|/Game/Blueprints/BP_SaveGame.BP_SaveGame_C|GetDialogueDone _savegame) (Variables|Default|GetSpeakerName)))
        (Variables|Default|SetNewArmor true)
        (Variables|Default|SetDialogueProgress (Utilities|Map|MakeMap 0 0 1 0))))
    (:else)))

(event EventTick
  (params (DeltaSeconds :type Float%20%28single-precision%29))
  (|CallParentFunction DeltaSeconds) ; This node is disabled and will not be called.\nDrag off pins to build functionality.
)

(fn Dialogue
  (|CallParentFunction)
  (bind (_dialoguestate _optionindex) (CallFunction|AddDialogue "Tajemniczy" "Widzę, że jednak udało ci się przeżyć walkę z tym potworem. Miałem 
wątpliwości, co do twoich umiejętności, ale widocznie cię nie doceniłem. Dalej ci będzie ciężko 
przetrwać, ale ku twojemu szczęściu mam coś co by Ci pomogło. Ale nie mogę Ci to oddać  
tak po prostu, musisz dać coś wzamian. Hmmmm, na przykład skóre pokonanego pająka. Co powiesz?" (Utilities|Array|MakeArray "Tak" "Nie") "/Game/Assets/Dubbing/Furys_pocz.Furys_pocz" false))
  (switch Utilities|FlowControl|Switch|SwitchonE_DialogueState _dialoguestate
    (:NewEnumerator0
      (bind _dialoguestate_2 (CallFunction|AddDialogue "" (Utilities|Array|Get(acopy) (Utilities|Array|MakeArray "Jeśli tak mówisz...Nie wiem co bym mogła zrobić z tą skórą, więc jeśli mogę wymienić 
ją na coś pomocnego tozgodzę się na twoją propozycje." "Nie rozumiem o czym ty gadasz. Nie mam żadnej skóry.") _optionindex) (Utilities|Array|MakeArray "[dalej]") (Utilities|Array|Get(acopy) (Utilities|Array|MakeArray "/Game/Assets/Dubbing/Tak.Tak" "/Game/Assets/Dubbing/Nie.Nie") _optionindex) true))
      (switch Utilities|FlowControl|Switch|SwitchonE_DialogueState _dialoguestate_2
        (:NewEnumerator0
          (switch int _optionindex
            (:0
              (bind _asbp_game_instance (Utilities|Casting|CastToBP_GameInstance (Game|GetGameInstance)))
              (bind _savegame (Variables|/Game/Blueprints/System/BP_GameInstance.BP_GameInstance_C|GetSaveGame _asbp_game_instance)
                (:then
                  (Utilities|Map|Add (Variables|/Game/Blueprints/BP_SaveGame.BP_SaveGame_C|GetDialogueDone _savegame) (Variables|Default|GetSpeakerName) true)
                  (if (not (Variables|Default|GetNewArmor))
                    (bind _asbp_hero_character (Utilities|Casting|CastToBP_HeroCharacter (Game|Player|GetPlayerPawn 0))
                      (:then
                        (Default|SetNewSkin _asbp_hero_character (Variables|/Game/Blueprints/Character/BP_HeroCharacter.BP_HeroCharacter_C|GetRogue _asbp_hero_character))
                        (Utilities|Array|AddUnique (Variables|/Game/Blueprints/Character/BP_HeroCharacter.BP_HeroCharacter_C|GetKeys _asbp_hero_character) 7))
                      (:CastFailed
                        _))))
                (:else
                  _))
              (bind _dialoguestate_3 (CallFunction|AddDialogue "Tajemniczy" "Wiedziałem, że jesteś rozsądną osobą." (Utilities|Array|MakeArray "[koniec]") "/Game/Assets/Dubbing/furys_tak.furys_tak" true))
              (switch Utilities|FlowControl|Switch|SwitchonE_DialogueState _dialoguestate_3
                (:NewEnumerator0
                  (CallFunction|RemoveDialogueProgress)
                  (CallFunction|CloseConversation))))
            (:1
              (bind _dialoguestate_4 (CallFunction|AddDialogue "Tajemniczy" "Mhm. Jak chcesz." (Utilities|Array|MakeArray "[koniec]") "/Game/Assets/Dubbing/furys_nie.furys_nie" true))
              (switch Utilities|FlowControl|Switch|SwitchonE_DialogueState _dialoguestate_4
                (:NewEnumerator0
                  (CallFunction|ClearDialogueProgress)
                  (CallFunction|CloseConversation))))))))))