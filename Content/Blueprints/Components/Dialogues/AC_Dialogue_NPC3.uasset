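; Dialogue component for NPC3 that delivers a single line of conversation and then ends it.
; The Dialogue override calls its parent, then adds one entry using the speaker, text and sound variables, with auto pass-through and a lone "[koniec]" (end) option.
; On the Pass Through state it clears dialogue progress and closes the conversation.
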(event EventBeginPlay
  (|CallParentFunction) ; This node is disabled and will not be called.\nDrag off pins to build functionality.
)

(event EventTick
  (params (DeltaSeconds :type Float%20%28single-precision%29))
  (|CallParentFunction DeltaSeconds) ; This node is disabled and will not be called.\nDrag off pins to build functionality.
)

(fn Dialogue
  (|CallParentFunction)
  (bind _dialoguestate (CallFunction|AddDialogue (Variables|Default|GetInSpeaker) (Variables|Default|GetInDialogue) (Utilities|Array|MakeArray "[koniec]") (Variables|Default|GetInSound) true))
  (switch Utilities|FlowControl|Switch|SwitchonE_DialogueState _dialoguestate
    (:NewEnumerator0
      (CallFunction|ClearDialogueProgress)
      (CallFunction|CloseConversation))))