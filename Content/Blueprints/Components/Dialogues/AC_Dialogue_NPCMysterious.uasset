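; Dialogue component for the mysterious NPC "Tajemniczy", scripting a short Polish conversation in which the NPC answers the player's questions only with "...".
; The Dialogue override calls its parent, then runs a linear chain of AddDialogue steps gated on Pass Through.
; Each chosen question is replayed as an auto-advancing line with a voice clip.
; The final option clears dialogue progress and closes the conversation.
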(event EventBeginPlay
  (|CallParentFunction) ; This node is disabled and will not be called.\nDrag off pins to build functionality.
)

(event EventTick
  (params (DeltaSeconds :type Float%20%28single-precision%29))
  (|CallParentFunction DeltaSeconds) ; This node is disabled and will not be called.\nDrag off pins to build functionality.
)

(fn Dialogue
  (bind _array (Utilities|Array|MakeArray "Cześć, jesteś może stąd?"))
  (bind _array_2 (Utilities|Array|MakeArray "Czy wiesz coś o tym miejscu?"))
  (|CallParentFunction)
  (bind (_dialoguestate _optionindex) (CallFunction|AddDialogue "Tajemniczy" "" _array 0 false))
  (switch Utilities|FlowControl|Switch|SwitchonE_DialogueState _dialoguestate
    (:NewEnumerator0
      (bind _dialoguestate_2 (CallFunction|AddDialogue "" (Utilities|Array|Get(acopy) _array _optionindex) (Utilities|Array|MakeArray "[dalej]") "/Game/Assets/Dubbing/Dziewczyna1.Dziewczyna1" true))
      (switch Utilities|FlowControl|Switch|SwitchonE_DialogueState _dialoguestate_2
        (:NewEnumerator0
          (bind _dialoguestate_3 (CallFunction|AddDialogue "Tajemniczy" "..." _array_2 0 false))
          (switch Utilities|FlowControl|Switch|SwitchonE_DialogueState _dialoguestate_3
            (:NewEnumerator0
              (bind _dialoguestate_4 (CallFunction|AddDialogue "" (Utilities|Array|Get(acopy) _array_2) (Utilities|Array|MakeArray "[dalej]") "/Game/Assets/Dubbing/Dziewczyna1_2.Dziewczyna1_2" true))
              (switch Utilities|FlowControl|Switch|SwitchonE_DialogueState _dialoguestate_4
                (:NewEnumerator0
                  (bind _dialoguestate_5 (CallFunction|AddDialogue "Tajemniczy" "..." (Utilities|Array|MakeArray "[koniec]") 0 false))
                  (switch Utilities|FlowControl|Switch|SwitchonE_DialogueState _dialoguestate_5
                    (:NewEnumerator0
                      (CallFunction|ClearDialogueProgress)
                      (CallFunction|CloseConversation))))))))))))