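; Child dialogue component that scripts a branching test conversation for speaker "Jan", with placeholder lines, reply options and a sound per line.
; The Dialogue override calls the parent, then switches on DialogueTreeIndex to pick one of two trees.
; Nested AddDialogue calls branch on option index whenever their state is Pass Through.
; Endings advance the tree index, remove some progress or clear it, then close the conversation.
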(event EventBeginPlay
  (|CallParentFunction) ; This node is disabled and will not be called.\nDrag off pins to build functionality.
)

(event EventTick
  (params (DeltaSeconds :type Float%20%28single-precision%29))
  (|CallParentFunction DeltaSeconds) ; This node is disabled and will not be called.\nDrag off pins to build functionality.
)

(fn Dialogue
  (|CallParentFunction)
  (switch int (Variables|Default|GetDialogueTreeIndex)
    (:0
      (bind (_dialoguestate _optionindex) (CallFunction|AddDialogue "Jan" "Test tt" (Utilities|Array|MakeArray "Tt" "ttt") "/Game/Assets/Sounds/Abilities/A_Ability_FireBallCast01.A_Ability_FireBallCast01"))
      (switch Utilities|FlowControl|Switch|SwitchonE_DialogueState _dialoguestate
        (:NewEnumerator0
          (switch int _optionindex
            (:0
              (bind (_dialoguestate_2 _optionindex_2) (CallFunction|AddDialogue "Jan" "Tt hh" (Utilities|Array|MakeArray "HH" "hh") "/Game/Assets/Sounds/Abilities/A_Ability_MeteorImpact01.A_Ability_MeteorImpact01"))
              (switch Utilities|FlowControl|Switch|SwitchonE_DialogueState _dialoguestate_2
                (:NewEnumerator0
                  (switch int _optionindex_2
                    (:0
                      (bind _dialoguestate_3 (CallFunction|AddDialogue "Jan" "123" (Utilities|Array|MakeArray "HH") "/Game/Assets/Sounds/Weapons/Axe/A_Axe_Swing01.A_Axe_Swing01"))
                      (switch Utilities|FlowControl|Switch|SwitchonE_DialogueState _dialoguestate_3
                        (:NewEnumerator0
                          (CallFunction|SetDialogueTreeIndex 1)
                          (CallFunction|CloseConversation))))
                    (:1
                      (bind _dialoguestate_4 (CallFunction|AddDialogue "Jan" "456" (Utilities|Array|MakeArray "HH") "/Game/Assets/Sounds/Abilities/A_Ability_TimeSlow01.A_Ability_TimeSlow01"))
                      (switch Utilities|FlowControl|Switch|SwitchonE_DialogueState _dialoguestate_4
                        (:NewEnumerator0
                          (CallFunction|RemoveDialogueProgress 2)
                          (CallFunction|CloseConversation))))))))
            (:1
              (bind _dialoguestate_5 (CallFunction|AddDialogue "Jan" "ttt" (Utilities|Array|MakeArray "GG" "gg") "/Game/Assets/Sounds/Abilities/A_Ability_MeteorWhoosh_01.A_Ability_MeteorWhoosh_01"))
              (switch Utilities|FlowControl|Switch|SwitchonE_DialogueState _dialoguestate_5
                (:NewEnumerator0
                  (CallFunction|ClearDialogueProgress)
                  (CallFunction|CloseConversation))))))))
    (:1
      (bind _dialoguestate_6 (CallFunction|AddDialogue "Jan" "Test tt" (Utilities|Array|MakeArray "Tt") "/Game/Assets/Sounds/Character/A_Character_Effort01.A_Character_Effort01"))
      (switch Utilities|FlowControl|Switch|SwitchonE_DialogueState _dialoguestate_6
        (:NewEnumerator0
          (CallFunction|RemoveDialogueProgress 1)
          (CallFunction|CloseConversation))))))