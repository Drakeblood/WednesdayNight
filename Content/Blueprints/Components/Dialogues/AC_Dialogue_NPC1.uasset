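; Dialogue component for NPC1, a voiced Polish conversation in which the NPC tells of their homeland Ankenterry, the place Nidavelirr, and how they arrived after dying in a war.
; It overrides the parent Dialogue function as a linear chain of AddDialogue calls, each advancing on Pass Through.
; Each single player option is echoed as an auto-advancing voiced line before the NPC replies.
; The final line clears dialogue progress and closes the conversation.
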(event EventBeginPlay
  (|CallParentFunction) ; This node is disabled and will not be called.\nDrag off pins to build functionality.
)

(event EventTick
  (params (DeltaSeconds :type Float%20%28single-precision%29))
  (|CallParentFunction DeltaSeconds) ; This node is disabled and will not be called.\nDrag off pins to build functionality.
)

(fn Dialogue
  (bind _array (Utilities|Array|MakeArray "Przepraszam,  jesteś stąd?"))
  (bind _array_2 (Utilities|Array|MakeArray "Dziękuję"))
  (bind _array_3 (Utilities|Array|MakeArray "Wiesz coś o tym gdzie my jesteśmy?"))
  (bind _array_4 (Utilities|Array|MakeArray "Jak tutaj trafiłeś?"))
  (|CallParentFunction)
  (bind (_dialoguestate _optionindex) (CallFunction|AddDialogue "" "" _array 0 false))
  (switch Utilities|FlowControl|Switch|SwitchonE_DialogueState _dialoguestate
    (:NewEnumerator0
      (bind _dialoguestate_2 (CallFunction|AddDialogue "" (Utilities|Array|Get(acopy) _array _optionindex) (Utilities|Array|MakeArray "[dalej]") "/Game/Assets/Dubbing/Przepraszam__jesteś_stąd.Przepraszam__jesteś_stąd" true))
      (switch Utilities|FlowControl|Switch|SwitchonE_DialogueState _dialoguestate_2
        (:NewEnumerator0
          (bind _dialoguestate_3 (CallFunction|AddDialogue "NPC1" "Jestem z  Ankenterry. To miejsce, gdzie żyją smoki, elfy, krasnoludy i inne magiczne stworzenia. Nasz świat jest bardzo różnorodny i pełen tajemnic. Mamy piękne lasy, góry, morza i wiele innych niezwykłych miejsc. Wszystko jest pełne magii i mistycyzmu, co sprawia, że nasze życie jest bardzo nieprzewidywalne." _array_3 "/Game/Assets/Dubbing/Npc1.Npc1" false))
          (switch Utilities|FlowControl|Switch|SwitchonE_DialogueState _dialoguestate_3
            (:NewEnumerator0
              (bind _dialoguestate_4 (CallFunction|AddDialogue "" (Utilities|Array|Get(acopy) _array_3) (Utilities|Array|MakeArray "[dalej]") "/Game/Assets/Dubbing/Wiesz_coś_o_tym_gdzie_my_jesteśmy.Wiesz_coś_o_tym_gdzie_my_jesteśmy" true))
              (switch Utilities|FlowControl|Switch|SwitchonE_DialogueState _dialoguestate_4
                (:NewEnumerator0
                  (bind _dialoguestate_5 (CallFunction|AddDialogue "NPC1" "Wiem tylko, że miejsce to nazywa się Nidavelirr. Tutaj możesz spotkać wiele istot z różnych światów i epok. To wszystko co udało mi się dowiedzieć." _array_4 "/Game/Assets/Dubbing/Npc1_2.Npc1_2" false))
                  (switch Utilities|FlowControl|Switch|SwitchonE_DialogueState _dialoguestate_5
                    (:NewEnumerator0
                      (bind _dialoguestate_6 (CallFunction|AddDialogue "" (Utilities|Array|Get(acopy) _array_4) (Utilities|Array|MakeArray "[dalej]") "/Game/Assets/Dubbing/Jak_tutaj_trafiłeś.Jak_tutaj_trafiłeś" true))
                      (switch Utilities|FlowControl|Switch|SwitchonE_DialogueState _dialoguestate_6
                        (:NewEnumerator0
                          (bind _dialoguestate_7 (CallFunction|AddDialogue "NPC1" "W moim kraju wybuchła wojna. Ankerterra jest bardzo złożona i pełna różnych ras, co czasem prowadzi do konfliktów. Ostatnie co pamiętam to strzałą przebijająca moje ciało, po tym  zapadła ciemność. Nie wiem ile czasu minęło i co dokładnie się stało, ale kiedy się obudziłem wszystko wokół mnie się zmieniło." _array_2 "/Game/Assets/Dubbing/Npc1_3.Npc1_3" false))
                          (switch Utilities|FlowControl|Switch|SwitchonE_DialogueState _dialoguestate_7
                            (:NewEnumerator0
                              (bind _dialoguestate_8 (CallFunction|AddDialogue "" (Utilities|Array|Get(acopy) _array_2) (Utilities|Array|MakeArray "[dalej]") "/Game/Assets/Dubbing/Dziękuję.Dziękuję" true))
                              (switch Utilities|FlowControl|Switch|SwitchonE_DialogueState _dialoguestate_8
                                (:NewEnumerator0
                                  (CallFunction|ClearDialogueProgress)
                                  (CallFunction|CloseConversation))))))))))))))))))