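; MoveToTargetNS is an anim notify state that pulls an AI character toward its follow target during an animation.
; Each tick it reads TargetToFollow from the AI controller's blackboard, then interpolates rotation to face it and location to a point 100 units short of it, with sweep.
; Movement is skipped while the player's BP_HeroCharacter is stopping time.
; A debug sphere for the destination is left disconnected.
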(fn ReceivedNotifyTick
  (params (MeshComp :type Skeletal%20Mesh%20Component%20Object%20Reference) (Animation :type Anim%20Sequence%20Base%20Object%20Reference) (FrameDeltaTime :type Float%20%28single-precision%29))
  (LocalVariables|SetMe (Components|GetOwner MeshComp))
  (bind _asbp_hero_character (Utilities|Casting|CastToBP_HeroCharacter (Game|Player|GetPlayerPawn MeshComp)))
  (if (not (Variables|/Game/Blueprints/Character/BP_HeroCharacter.BP_HeroCharacter_C|GetIsStoppingTime _asbp_hero_character))
    (Utilities|IsValid (AI|GetAIController (LocalVariables|GetMe))
      (:Is%20Valid
        (bind _asactor (Utilities|Casting|CastToActor (AI|Components|Blackboard|GetValueasObject (Variables|/Script/AIModule.AIController|GetBlackboard (AI|GetAIController (LocalVariables|GetMe))) (Utilities|Name|MakeLiteralName "TargetToFollow"))))
        (LocalVariables|SetTarget _asactor)
        (Transformation|SetActorRotation (LocalVariables|GetMe) (Math|Interpolation|RInterpTo (Transformation|GetActorRotation (LocalVariables|GetMe)) (Math|Rotator|FindLookatRotation (Transformation|GetActorLocation (LocalVariables|GetMe)) (Transformation|GetActorLocation (LocalVariables|GetTarget))) (Utilities|Time|GetWorldDeltaSeconds (LocalVariables|GetMe)) (Variables|Default|GetRotationInterpSpeed)))
        (Transformation|SetActorLocation (LocalVariables|GetMe) (Math|Interpolation|VInterpTo (Transformation|GetActorLocation (LocalVariables|GetMe)) (+ (Transformation|GetActorLocation (LocalVariables|GetTarget)) (* (Math|Vector|GetForwardVector (Math|Rotator|FindLookatRotation (Transformation|GetActorLocation (LocalVariables|GetMe)) (Transformation|GetActorLocation (LocalVariables|GetTarget)))) -1e+02)) (Utilities|Time|GetWorldDeltaSeconds (LocalVariables|GetMe)) (Variables|Default|GetLocationInterpSpeed)) true false)
        (return true)))))