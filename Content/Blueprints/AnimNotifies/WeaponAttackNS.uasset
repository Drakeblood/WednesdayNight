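; WeaponAttackNS is an animation notify state that marks the attack window of a character's current weapon during an animation.
; On begin, it casts the mesh owner to BP_CharacterBase, sets IsAttacking on a valid CurrentWeapon and calls its EventBeginWeaponAttack.
; On end, it calls EventEndWeaponAttack on that character's current weapon, without clearing IsAttacking itself.
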(fn ReceivedNotifyBegin
  (params (MeshComp :type Skeletal%20Mesh%20Component%20Object%20Reference) (Animation :type Anim%20Sequence%20Base%20Object%20Reference) (TotalDuration :type Float%20%28single-precision%29))
  (bind _asbp_character_base (Utilities|Casting|CastToBP_CharacterBase (Components|GetOwner MeshComp)))
  (Utilities|IsValid (Variables|/Game/Blueprints/Character/BP_CharacterBase.BP_CharacterBase_C|GetCurrentWeapon _asbp_character_base)
    (:Is%20Valid
      (Variables|/Game/Blueprints/Weapon/WeaponActor.WeaponActor_C|SetIsAttacking (Variables|/Game/Blueprints/Character/BP_CharacterBase.BP_CharacterBase_C|GetCurrentWeapon _asbp_character_base) true)
      (Default|EventBeginWeaponAttack (Variables|/Game/Blueprints/Character/BP_CharacterBase.BP_CharacterBase_C|GetCurrentWeapon _asbp_character_base))
      (return true))))

(fn ReceivedNotifyEnd
  (params (MeshComp :type Skeletal%20Mesh%20Component%20Object%20Reference) (Animation :type Anim%20Sequence%20Base%20Object%20Reference))
  (bind _asbp_character_base (Utilities|Casting|CastToBP_CharacterBase (Components|GetOwner MeshComp)))
  (Utilities|IsValid (Variables|/Game/Blueprints/Character/BP_CharacterBase.BP_CharacterBase_C|GetCurrentWeapon _asbp_character_base)
    (:Is%20Valid
      (Default|EventEndWeaponAttack (Variables|/Game/Blueprints/Character/BP_CharacterBase.BP_CharacterBase_C|GetCurrentWeapon _asbp_character_base))
      (return false))))