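; Player controller Blueprint that owns the player's HUD and menu widgets.
; On possess, it creates the HUD and adds it to the viewport, and creates the menu widget without showing it.
; A ShowGameOverMenu event later adds that stored menu to the viewport and makes its game-over text visible.
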(event Custom|ShowGameOverMenu
  (bind _menuwidget (Variables|Default|GetMenuWidget))
  (UserInterface|Viewport|AddtoViewport _menuwidget 0)
  (Widget|SetVisibility (Variables|/Game/Blueprints/UI/WBP_Menu.WBP_Menu_C|GetGameOverText _menuwidget) "Visible"))

(event EventPossess
  (params (PossessedPawn :type Pawn%20Object%20Reference))
  (bind _returnvalue (UserInterface|CreateWidget "/Game/Blueprints/UI/WBP_HUD.WBP_HUD_C" self))
  (bind _output_get (Variables|Default|SetPlayerHUDWidget _returnvalue))
  (UserInterface|Viewport|AddtoViewport _output_get 0)
  (bind _returnvalue_2 (UserInterface|CreateWidget "/Game/Blueprints/UI/WBP_Menu.WBP_Menu_C" self))
  (Variables|Default|SetMenuWidget _returnvalue_2))

(fn ConstructionScript)