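; BP_InteractableDoor2 is a key-locked door that slides open and closed when interacted with.
; Its availability check passes only for a BP_HeroCharacter whose Keys contain the door's KeyID.
; AC_Interaction toggles a FlipFlop that plays the OpenCloseDoor timeline from start or reverses it from end, lerping the actor between its starting location and a local offset converted to world space at BeginPlay.
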(event OnInteract(AC_Interaction)
  (params (Interacter :type Actor%20Object%20Reference))
  (Utilities|FlowControl|FlipFlop
    (:A
      (Development|PrintString "Hello")
      (bind _alpha (Timeline|OpenCloseDoor PlayFromStart)
        (:Update
          (Transformation|SetActorLocation (Math|Vector|Lerp(Vector) (Variables|Default|GetOriginalLocation) (Variables|Default|GetOnActivateWorldLocation) _alpha) false false))))
    (:B
      (Timeline|OpenCloseDoor ReverseFromEnd))))

(event EventBeginPlay
  (Variables|Default|SetOriginalLocation (Transformation|GetActorLocation))
  (Variables|Default|SetOnActivateWorldLocation (Math|Transform|TransformLocation (Transformation|GetActorTransform) (Variables|Default|GetOnActivateLocation))))

(fn ConstructionScript)

(fn IsAvailableforInteraction
  (params (Interacter :type Actor%20Object%20Reference))
  (bind _asbp_hero_character (Utilities|Casting|CastToBP_HeroCharacter Interacter)
    (:then
      (return (Utilities|Array|ContainsItem (Variables|/Game/Blueprints/Character/BP_HeroCharacter.BP_HeroCharacter_C|GetKeys _asbp_hero_character) (Variables|Default|GetKeyID))))
    (:CastFailed
      (return false))))