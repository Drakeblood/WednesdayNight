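; Interactable door that swings open and closed on alternate interactions, available only to a hero character holding its key.
; AC_Interaction's OnInteract drives a FlipFlop that plays or reverses the OpenCloseDoor timeline, whose Alpha lerps the mesh's relative yaw a quarter turn, with Inverse choosing the direction.
; IsAvailableForInteraction casts the interacter to BP_HeroCharacter and checks its Keys for the door's KeyID, rejecting anyone else.
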(event OnInteract(AC_Interaction)
  (params (Interacter :type Actor%20Object%20Reference))
  (Utilities|FlowControl|FlipFlop
    (:A
      (bind _alpha (Timeline|OpenCloseDoor PlayFromStart)
        (:Update
          (Transformation|SetRelativeRotation (Variables|Default|GetStaticMesh) (Math|Rotator|MakeRotator 0.0 0.0 (Math|Float|Lerp 0.0 (Math|Float|SelectFloat -9e+01 9e+01 (Variables|Default|GetInverse)) _alpha)) false false))))
    (:B
      (Timeline|OpenCloseDoor ReverseFromEnd))))

(fn ConstructionScript)

(fn IsAvailableforInteraction
  (params (Interacter :type Actor%20Object%20Reference))
  (bind _asbp_hero_character (Utilities|Casting|CastToBP_HeroCharacter Interacter)
    (:then
      (return (Utilities|Array|ContainsItem (Variables|/Game/Blueprints/Character/BP_HeroCharacter.BP_HeroCharacter_C|GetKeys _asbp_hero_character) (Variables|Default|GetKeyID))))
    (:CastFailed
      (return false))))