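; An interactable save point that writes the hero's progress to disk when used.
; On interact it reuses the SaveGame held by BP_GameInstance, or creates a BP_SaveGame and caches it there.
; It records the hero's health and max health, the PlayerSpawn transform as the respawn location and rotation, and the game mode's LorePoint when available, then saves to a fixed slot.
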(event OnInteract(AC_Interaction)
  (params (Interacter :type Actor%20Object%20Reference))
  (bind _playerspawn (Variables|Default|GetPlayerSpawn))
  (bind _returnvalue (Transformation|GetWorldTransform _playerspawn))
  (bind _asbp_hero_character (Utilities|Casting|CastToBP_HeroCharacter Interacter))
  (bind _asbp_game_instance (Utilities|Casting|CastToBP_GameInstance (Game|GetGameInstance)))
  (bind _savegame (Variables|/Game/Blueprints/System/BP_GameInstance.BP_GameInstance_C|GetSaveGame _asbp_game_instance)
    (:then
      (Variables|Default|SetSaveGame _savegame))
    (:else
      (bind _returnvalue_2 (SaveGame|CreateSaveGameObject "/Game/Blueprints/BP_SaveGame.BP_SaveGame_C"))
      (bind _output_get (Variables|Default|SetSaveGame _returnvalue_2))
      (Variables|/Game/Blueprints/System/BP_GameInstance.BP_GameInstance_C|SetSaveGame _asbp_game_instance _output_get)))
  (Variables|/Game/Blueprints/BP_SaveGame.BP_SaveGame_C|SetHealth (Variables|Default|GetSaveGame) (Default|GetHealth (Variables|/Game/Blueprints/Character/BP_CharacterBase.BP_CharacterBase_C|GetAttributes _asbp_hero_character)))
  (Variables|/Game/Blueprints/BP_SaveGame.BP_SaveGame_C|SetMaxHealth (Variables|Default|GetSaveGame) (Default|GetMaxHealth (Variables|/Game/Blueprints/Character/BP_CharacterBase.BP_CharacterBase_C|GetAttributes _asbp_hero_character)))
  (Variables|/Game/Blueprints/BP_SaveGame.BP_SaveGame_C|SetSpawnLocation (Variables|Default|GetSaveGame) (.location _returnvalue))
  (Variables|/Game/Blueprints/BP_SaveGame.BP_SaveGame_C|SetSpawnRotation (Variables|Default|GetSaveGame) (.rotation _returnvalue))
  (bind _asbp_game_mode (Utilities|Casting|CastToBP_GameMode (Game|GetGameMode))
    (:then
      (Variables|/Game/Blueprints/BP_SaveGame.BP_SaveGame_C|SetLorePoint (Variables|Default|GetSaveGame) (Variables|/Game/Blueprints/GameModes/BP_GameMode.BP_GameMode_C|GetLorePoint _asbp_game_mode)))
    (:CastFailed
      _))
  (SaveGame|SaveGametoSlot (Variables|Default|GetSaveGame) "Slot0"))

(fn ConstructionScript)