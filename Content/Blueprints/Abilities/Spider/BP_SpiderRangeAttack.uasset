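; BP_SpiderRangeAttack is a spider ability that fires a BP_SpiderProjectile at the player.
; When added to a BP_Spider, it sets the projectile scale to half size.
; On a "Projectile" anim notify, it spawns the projectile from the mesh's ProjectileSocket with the character as owner and instigator.
; Aim leads the player by offsetting their location with velocity times a distance-based travel-time estimate.
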(event EventOnNotifyBegin
  (params (NotifyName :type Name :default "None"))
  (if (Utilities|Name|Equal(Name) NotifyName "Projectile")
    (bind _asbp_character_base (Utilities|Casting|CastToBP_CharacterBase (CallFunction|GetAvatarActor)))
    (Default|SpawnActor _asbp_character_base "/Game/Blueprints/Weapon/BP_SpiderProjectile.BP_SpiderProjectile_C" (Math|Transform|MakeTransform (Transformation|GetSocketLocation (Variables|/Script/Engine.Character|GetMesh _asbp_character_base) "ProjectileSocket") (Math|Rotator|FindLookatRotation (Transformation|GetSocketLocation (Variables|/Script/Engine.Character|GetMesh _asbp_character_base) "ProjectileSocket") (+ (Transformation|GetActorLocation (Default|GetPlayer _asbp_character_base)) (* (Transformation|GetVelocity (Default|GetPlayer _asbp_character_base)) (/ (Transformation|GetDistanceTo _asbp_character_base (Default|GetPlayer _asbp_character_base)) 5e+03)))) (Variables|Default|GetProjectileScale)) "Undefined" _asbp_character_base _asbp_character_base)))

(event EventAbilityAdded
  (|CallParentFunction)
  (Utilities|Casting|CastToBP_Spider (CallFunction|GetAvatarActor))
  (Variables|Default|SetProjectileScale "0.500000,0.500000,0.500000"))