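; Ice Golem boss special attack ability that spawns attack actors in response to named notifies.
; SpecialAttack1 spawns an Aqua Storm at the boss's AquaStormLocation, converted from local to world space through its transform.
; SpecialAttack2 spawns a Rock Rain at the level's BP_RainLocation actor.
; Both spawns require an Ice Golem boss avatar and set it as owner and instigator.
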(event EventOnNotifyBegin
  (params (NotifyName :type Name :default "None"))
  (bind _avataractor (CallFunction|GetAvatarActor))
  (if (Utilities|Name|Equal(Name) NotifyName "SpecialAttack1")
    (bind _asbp_ice_golem_boss (Utilities|Casting|CastToBP_IceGolemBoss _avataractor))
    (Default|SpawnActor _asbp_ice_golem_boss "/Game/Blueprints/Weapon/Golem/BP_GolemAquaStorm.BP_GolemAquaStorm_C" (Math|Transform|MakeTransform (Math|Transform|TransformLocation (Transformation|GetActorTransform _asbp_ice_golem_boss) (Variables|/Game/Blueprints/Enemy/BP_IceGolemBoss.BP_IceGolemBoss_C|GetAquaStormLocation _asbp_ice_golem_boss)) "0, 0, 0" "1,1,1") "Undefined" _asbp_ice_golem_boss _asbp_ice_golem_boss)
    (elif (Utilities|Name|Equal(Name) NotifyName "SpecialAttack2")
      (bind _asbp_ice_golem_boss_2 (Utilities|Casting|CastToBP_IceGolemBoss _avataractor))
      (Default|SpawnActor _asbp_ice_golem_boss_2 "/Game/Blueprints/Weapon/Golem/BP_GolemRockRain.BP_GolemRockRain_C" (Math|Transform|MakeTransform (Transformation|GetActorLocation (Default|GetActorOfClass _asbp_ice_golem_boss_2 "/Game/Blueprints/Weapon/Golem/BP_RainLocation.BP_RainLocation_C")) "0, 0, 0" "1,1,1") "Undefined" _asbp_ice_golem_boss_2 _asbp_ice_golem_boss_2))))