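; BP_NPC is an interactable NPC that opens a conversation when a player interacts with it.
; AC_Interaction's OnInteract calls OpenConversation on the AC_DialogueBase component, then switches the interacting hero's player controller to UI-only input and shows the cursor.
; BeginPlay caches a dialog row from DialogRowHandle in CurrentDialog, which only an unconnected WBP_Dialog widget chain reads in this graph.
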(event OnInteract(AC_Interaction)
  (params (Interacter :type Actor%20Object%20Reference))
  (Default|OpenConversation (Actor|GetComponentbyClass "/Game/Blueprints/Components/AC_DialogueBase.AC_DialogueBase_C"))
  (bind _asbp_hero_character (Utilities|Casting|CastToBP_HeroCharacter Interacter))
  (bind _asbp_player_controller (Utilities|Casting|CastToBP_PlayerController (Pawn|GetController _asbp_hero_character)))
  (Input|SetInputModeUIOnly _asbp_player_controller 0 "DoNotLock")
  (Variables|/Script/Engine.PlayerController|SetbShowMouseCursor _asbp_player_controller true))

(event EventBeginPlay
  (bind _dialogrowhandle (Variables|Default|GetDialogRowHandle))
  (|CallParentFunction)
  (bind _returnvalue (Utilities|GetDataTableRow (.datatable _dialogrowhandle) (.rowname _dialogrowhandle))
    (:then
      (Variables|Default|SetCurrentDialog _returnvalue))))

(event Collision|EventActorBeginOverlap
  (params (OtherActor :type Actor%20Object%20Reference)))

(event EventTick
  (params (DeltaSeconds :type Float%20%28single-precision%29)))

(fn ConstructionScript
  (|CallParentFunction))