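; BP_CharacterBase is a character base Blueprint that handles damage, hit reactions and death.
; Any damage lowers health on the Attributes component, whose change event calls Death at zero or below to disable actor collision.
; Hit-react montages are throttled by a small counter, apparently restored by a timer, and are skipped while a high-priority montage plays.
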(event OnHealthChanged(Attributes)
  (params (NewHealth :type Float%20%28single-precision%29) (AttributesComponent :type AC%20Attributes%20Object%20Reference))
  (if (<= NewHealth 0.0)
    (CallFunction|Death)))

(event Custom|Death
  (Collision|SetActorEnableCollision false))

(event Custom|ResetHitReactBuffor
  (Variables|Montages|SetHitReactBuffor 2))

(event Custom|OnTakeAnyDamage_Event
  (params (DamagedActor :type Actor%20Object%20Reference) (Damage :type Float%20%28single-precision%29) (DamageType :type Damage%20Type%20Object%20Reference) (InstigatedBy :type Controller%20Object%20Reference) (DamageCauser :type Actor%20Object%20Reference))
  (bind _attributes (Variables|Default|GetAttributes))
  (if (or (CallFunction|IsPlayingHighPriorityMontage) (< (Variables|Montages|GetHitReactBuffor) 1))
    _
    (else
      (Animation|Montage|PlayMontage (Variables|Character|GetMesh) (Variables|Montages|GetHitReactMontage)
        (:then
          (Math|Integer|DecrementInt (Variables|Montages|GetHitReactBuffor)
            (:%20%20
              (Utilities|Time|SetTimerbyEvent (EventDispatchers|CreateEvent :!event Custom|ResetHitReactBuffor) 2.0)))))))
  (Default|SetHealth _attributes (- (Default|GetHealth _attributes) Damage)))

(event EventBeginPlay
  (EventDispatchers|AssignOnTakeAnyDamage (delegate Custom|OnTakeAnyDamage_Event)))

(fn ConstructionScript)

(fn IsPlayingHighPriorityMontage
  (LocalVariables|SetAnimInstance (Components|SkeletalMesh|GetAnimInstance (Variables|Character|GetMesh)))
  (if (Class|AnimInstance|IsAnyMontagePlaying (LocalVariables|GetAnimInstance))
    (for _array_element (Variables|Montages|GetHighPriorityMontages)
      (if (Animation|Montage|MontageIsPlaying (LocalVariables|GetAnimInstance) _array_element)
        (return true)))
    (return false)
    (else
      (return false))))