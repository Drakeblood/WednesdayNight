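; NPC_SpiderBoss is a spider boss NPC Blueprint whose events (BeginPlay, damage, death, hit effect) are all empty stubs.
; Disconnected, never-executed logic would attach a BP_WeaponSpider to the front-right knee socket and remove the shadow before delayed destruction.
; Other dead fragments play randomly chosen hit montage sections for root motion, call the hit effect and reset a "Hit" material parameter.
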(event Custom|SpiderBossHitEffect)

(event Custom|OnDamaged_1)

(event Custom|OnDeathEvent_1)

(event EventBeginPlay)

(fn ConstructionScript)