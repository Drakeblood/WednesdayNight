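; BP_GolemAquaStorm is a golem attack, a storm that chases the player hero and damages them on contact.
; Tick moves it toward the hero using look-at yaw with pitch zeroed, pausing while the hero stops time.
; After a delay from BeginPlay, a timeline lowers it from its current location.
; Box overlap applies damage, disables overlaps briefly, then nudges and restores the box position to refresh overlap detection.
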(event OnComponentBeginOverlap(Box)
  (params (OverlappedComponent :type Primitive%20Component%20Object%20Reference) (OtherActor :type Actor%20Object%20Reference) (OtherComp :type Primitive%20Component%20Object%20Reference) (OtherBodyIndex :type Integer) (bFromSweep :type Boolean) (SweepResult :type Hit%20Result%20Structure%20%28by%20ref%29))
  (bind _box (Variables|Default|GetBox))
  (bind _box_2 (Variables|Default|GetBox))
  (bind _relativelocation (Variables|/Script/Engine.SceneComponent|GetRelativeLocation _box_2))
  (bind _asbp_hero_character (Utilities|Casting|CastToBP_HeroCharacter OtherActor))
  (Game|Damage|ApplyDamage _asbp_hero_character 1e+01 (Pawn|GetController (Game|GetInstigator)) self)
  (Variables|/Script/Engine.PrimitiveComponent|SetbGenerateOverlapEvents (Variables|Default|GetBox) false)
  (Utilities|FlowControl|Delay 1.5)
  (bind _output_get (Variables|Default|SetOriginalRelativeLocation _relativelocation))
  (Transformation|SetRelativeLocation _box_2 (+ _relativelocation 0.1) false false)
  (Variables|/Script/Engine.PrimitiveComponent|SetbGenerateOverlapEvents _box true)
  (Transformation|SetRelativeLocation _box _output_get false false))

(event EventBeginPlay
  (bind _returnvalue (Transformation|GetActorLocation))
  (Variables|Default|SetHero (Game|Player|GetPlayerPawn 0))
  (Utilities|FlowControl|Delay 9.0)
  (bind _newtrack_0 (Timeline|Timeline_0 PlayFromStart)
    (:Update
      (Transformation|SetActorLocation (Math|Vector|Lerp(Vector) _returnvalue (+ _returnvalue "0, 0,-200.000000") _newtrack_0) false false))))

(event Collision|EventActorBeginOverlap
  (params (OtherActor :type Actor%20Object%20Reference)))

(event EventTick
  (params (DeltaSeconds :type Float%20%28single-precision%29))
  (bind _returnvalue (Transformation|GetActorLocation))
  (bind _hero (Variables|Default|GetHero))
  (bind _returnvalue_2 (Transformation|GetActorLocation _hero))
  (bind _returnvalue_3 (Math|Rotator|FindLookatRotation _returnvalue _returnvalue_2))
  (bind _asbp_hero_character (Utilities|Casting|CastToBP_HeroCharacter (Variables|Default|GetHero)))
  (if (not (Variables|/Game/Blueprints/Character/BP_HeroCharacter.BP_HeroCharacter_C|GetIsStoppingTime _asbp_hero_character))
    (Transformation|AddActorLocalOffset (* (Math|Vector|Normalize (Math|Rotator|GetRotationXVector (Math|Rotator|MakeRotator (.roll _returnvalue_3) 0.0 (.yaw _returnvalue_3)))) (* DeltaSeconds 4e+02)) false false)))

(fn ConstructionScript)