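; BP_GolemRockRain is a golem attack actor that rains BP_IceGolemProjectile rocks on the player.
; After a short delay it loops every second, spawning a projectile at a random point in its Box.
; Each is aimed ahead of the hero's velocity, with lead time based on instigator-to-hero distance and projectile speed.
; Box overlap damages the hero, then disables overlap events; the re-enable logic is unwired, so it hits once.
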(event OnComponentBeginOverlap(Box)
  (params (OverlappedComponent :type Primitive%20Component%20Object%20Reference) (OtherActor :type Actor%20Object%20Reference) (OtherComp :type Primitive%20Component%20Object%20Reference) (OtherBodyIndex :type Integer) (bFromSweep :type Boolean) (SweepResult :type Hit%20Result%20Structure%20%28by%20ref%29))
  (bind _asbp_hero_character (Utilities|Casting|CastToBP_HeroCharacter OtherActor))
  (Game|Damage|ApplyDamage _asbp_hero_character 1e+01 (Pawn|GetController (Game|GetInstigator)) self)
  (Variables|/Script/Engine.PrimitiveComponent|SetbGenerateOverlapEvents (Variables|Default|GetBox) false)
  (Utilities|FlowControl|Delay 1.5))

(event Custom|SpawnRock
  (bind _box (Variables|Default|GetBox))
  (bind _hero (Variables|Default|GetHero))
  (bind _output_get (Variables|Default|SetRandomLocation (Math|Random|RandomPointinBoundingBox (Transformation|GetWorldLocation _box) (Variables|/Script/Engine.BoxComponent|GetBoxExtent _box))))
  (Game|SpawnActorfromClass "/Game/Blueprints/Weapon/Golem/BP_IceGolemProjectile.BP_IceGolemProjectile_C" (Math|Transform|MakeTransform _output_get (Math|Rotator|FindLookatRotation _output_get (+ (Transformation|GetActorLocation _hero) (* (Transformation|GetVelocity _hero) (/ (Transformation|GetDistanceTo (.AsBP%20Character%20Base (Utilities|Casting|CastToBP_CharacterBase (Game|GetInstigator))) _hero) 2e+03)))) "1,1,1") "AdjustIfPossibleButDontSpawnIfColliding" self 2e+03 0))

(event EventBeginPlay
  (Variables|Default|SetHero (Game|Player|GetPlayerPawn 0))
  (Utilities|FlowControl|Delay 0.5)
  (CallFunction|SpawnRock :!label _label)
  (Utilities|FlowControl|Delay 1.0)
  (goto _label))

(fn ConstructionScript)