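; Melee weapon actor that deals damage to actors its capsule overlaps during an attack.
; Begin and end attack events toggle query-only capsule collision and an attacking flag, with a short delay before switching off.
; Overlaps during an attack skip actors of the instigator's class and use a unique-add hit list so each target takes damage once per swing, credited to the instigator's controller.
; The hit list clears when the attack ends.
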(event Custom|Event%20BeginWeaponAttack
  (Variables|WeaponDefaults|SetIsAttacking true)
  (Collision|SetCollisionEnabled (Variables|Default|GetCapsuleCollision) "QueryOnly"))

(event Custom|Event%20EndWeaponAttack
  (Utilities|FlowControl|Delay 0.2)
  (Variables|WeaponDefaults|SetIsAttacking false)
  (Collision|SetCollisionEnabled (Variables|Default|GetCapsuleCollision) "NoCollision")
  (Utilities|Array|Clear (Variables|Default|GetHitActors)))

(event Collision|EventActorBeginOverlap
  (params (OtherActor :type Actor%20Object%20Reference))
  (if (and (!= (Utilities|GetClass OtherActor) (Utilities|GetClass (Game|GetInstigator))) (Variables|WeaponDefaults|GetIsAttacking))
    (bind _returnvalue (Utilities|Array|AddUnique (Variables|Default|GetHitActors) OtherActor))
    (if (!= _returnvalue -1)
      (Game|Damage|ApplyDamage OtherActor (Variables|WeaponDefaults|GetWeaponDamage) (Pawn|GetController (Game|GetInstigator)) self))))

(event EventBeginPlay
  (Collision|IgnoreActorwhenMoving (Variables|Default|GetCapsuleCollision) 0 true))

(fn ConstructionScript)